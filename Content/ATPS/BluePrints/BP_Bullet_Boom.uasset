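; BP_Bullet_Boom is an explosive bullet that bursts when it hits something.
; On Hit, it spawns a particle effect at its location and runs a short multi sphere trace on Visibility around itself.
; Each BP_StaticMesh found gets one shared velocity, aimed from the hit point toward the struck actor's origin rather than radially outward.
; A delayed trigger into the same blast logic is left unconnected.
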(event EventBeginPlay
  (|CallParentFunction) ; 此节点被禁用，将不会被调用。\n从引脚连出引线来编译功能。
)

(event Collision|EventActorBeginOverlap
  (params (OtherActor :type Actor%20Object%20Reference))
  (|CallParentFunction OtherActor) ; 此节点被禁用，将不会被调用。\n从引脚连出引线来编译功能。
)

(event EventTick
  (params (DeltaSeconds :type Float%20%28single-precision%29))
  (|CallParentFunction DeltaSeconds) ; 此节点被禁用，将不会被调用。\n从引脚连出引线来编译功能。
)

(event Collision|EventHit
  (params (MyComp :type Primitive%20Component%20Object%20Reference) (Other :type Actor%20Object%20Reference) (OtherComp :type Primitive%20Component%20Object%20Reference) (bSelfMoved :type Boolean) (HitLocation :type Vector :default "0, 0, 0") (HitNormal :type Vector :default "0, 0, 0") (NormalImpulse :type Vector :default "0, 0, 0") (Hit :type Hit%20Result%20Structure%20%28by%20ref%29))
  (bind _returnvalue (Transformation|GetActorLocation))
  (Effects|SpawnEmitteratLocation "/Engine/Tutorial/SubEditors/TutorialAssets/TutorialParticleSystem.TutorialParticleSystem" _returnvalue)
  (bind _outhits (Collision|MultiSphereTraceByChannel _returnvalue (+ _returnvalue "0.000000, 0,10.000000") 1e+02 "TraceTypeQuery1" false 0 "ForOneFrame"))
  (for _array_element _outhits
    (bind _asbp_static_mesh (Utilities|Casting|CastToBP_StaticMesh (.hitactor _array_element)))
    (Default|SetVelocity _asbp_static_mesh (* (Math|Vector|Normalize (- (Transformation|GetActorLocation Other) HitLocation)) 3000))))

(fn ConstructionScript
  (|CallParentFunction))