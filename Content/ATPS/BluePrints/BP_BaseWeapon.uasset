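; Base weapon actor that a character can pick up, fire, reload and detach as a physics object.
; Firing plays the character's montage and spawns a bullet at the muzzle socket aimed at the owner's LookAtPoint, or shows a timed reload hint when empty.
; TagOfClass selects montage-driven regular bullets and reloads, or immediate explosive-type bullets and instant refills.
; Pickup disables physics and derives an aim offset from the sight socket.
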(event Custom|MagReloadWeapon
  (if (!= (Variables|Default|GetTagOfClass) 0)
    _
    (else
      (Animation|Montage|PlayMontage (Variables|Default|GetSkeletalMesh) "/Game/ATPS/Assets/Weapons/AM_AR_Reload_NoCharge.AM_AR_Reload_NoCharge"
        (:OnCompleted
          _))))
  (Variables|Default|SetRoundsinChamber (Variables|Default|GetMagSize)))

(event Custom|Detach
  (Transformation|DetachFromActor "KeepWorld" "KeepWorld" "KeepWorld")
  (Physics|SetSimulatePhysics (Variables|Default|GetSkeletalMesh) true)
  (Collision|SetCollisionEnabled (Variables|Default|GetSkeletalMesh) "QueryAndPhysics"))

(event EventBeginPlay)

(event Collision|EventActorBeginOverlap
  (params (OtherActor :type Actor%20Object%20Reference)))

(event EventTick
  (params (DeltaSeconds :type Float%20%28single-precision%29)))

(event EventFirePressed
  (bind _skeletalmesh (Variables|Default|GetSkeletalMesh))
  (bind _returnvalue (Transformation|GetSocketTransform _skeletalmesh "ShootStart" "RTS_World"))
  (if (> (Variables|Default|GetRoundsinChamber) 0)
    (Animation|Montage|PlayMontage (Variables|/Script/Engine.Character|GetMesh (Variables|Default|GetOwning%20Character)) "/Game/ATPS/Assets/Character/AM_2HW_ADS_Fire.AM_2HW_ADS_Fire"
      (:then
        (if (!= (Variables|Default|GetTagOfClass) 0)
          (bind _returnvalue_2 (Game|SpawnActorfromClass "/Game/ATPS/BluePrints/BP_Bullet_Boom.BP_Bullet_Boom_C" (Math|Transform|MakeTransform (.location _returnvalue) (.rotation _returnvalue) (.scale _returnvalue)) "AlwaysSpawn" 0 0))
          (CallFunction|SetVelocity _returnvalue_2)
          (else
            (Animation|Montage|PlayMontage (Variables|Default|GetSkeletalMesh) "/Game/ATPS/Assets/Weapons/AM_AR_Fire.AM_AR_Fire"
              (:OnNotifyBegin
                (bind _returnvalue_3 (Game|SpawnActorfromClass "/Game/ATPS/BluePrints/BP_Bullet.BP_Bullet_C" (Math|Transform|MakeTransform (.location _returnvalue) (.rotation _returnvalue) (.scale _returnvalue)) "AlwaysSpawn" 0 0))
                (CallFunction|SetVelocity _returnvalue_3)))))))
    (else
      (bind _asmy_player_controller (Utilities|Casting|CastToMyPlayerController (Game|GetPlayerController 0)))
      (Default|SetText (Variables|/Game/GamePlay/MyPlayerController.MyPlayerController_C|GetHelpWidgetOfR _asmy_player_controller) "请按R装弹")
      (UserInterface|Viewport|AddtoViewport (Variables|/Game/GamePlay/MyPlayerController.MyPlayerController_C|GetHelpWidgetOfR _asmy_player_controller) 0)
      (Utilities|FlowControl|Delay 0.8)
      (Widget|RemovefromParent (Variables|/Game/GamePlay/MyPlayerController.MyPlayerController_C|GetHelpWidgetOfR _asmy_player_controller)))))

(event EventGetWeapon
  (params (OwningCharacter :type BP%20Base%20Character%20Object%20Reference))
  (Variables|Default|SetOwning%20Character OwningCharacter)
  (Physics|SetSimulatePhysics (Variables|Default|GetSkeletalMesh) false)
  (Collision|SetCollisionEnabled (Variables|Default|GetSkeletalMesh) "NoCollision")
  (Variables|Default|SetAimBaselineOffset (- (Class|KismetAnimationLibrary|DistanceBetweenTwoSocketsandMapRange (Variables|Default|GetSkeletalMesh) "Root" "RTS_World" "Sight" "RTS_World" false 0.0 0.0 0.0 0.0) 21.0)))

(fn ConstructionScript)

(fn SetVelocity
  (params (Bullet :type BP%20Bullet%20Object%20Reference))
  (bind _output_get (Variables|/Game/ATPS/BluePrints/BP_Bullet.BP_Bullet_C|SetVelocity Bullet (* (Math|Vector|Normalize (- (Variables|/Game/ATPS/BluePrints/BP_BaseCharacter.BP_BaseCharacter_C|GetLookAtPoint (Variables|Default|GetOwning%20Character)) (Transformation|GetSocketLocation (Variables|Default|GetSkeletalMesh) "ShootStart"))) 3e+03)))
  (Variables|/Script/Engine.MovementComponent|SetVelocity (Variables|/Game/ATPS/BluePrints/BP_Bullet.BP_Bullet_C|GetBeenShooted Bullet) _output_get)
  (Variables|Default|SetRoundsinChamber (- (Variables|Default|GetRoundsinChamber) 1)))

(fn GetWeaponPanelInfo
  (return self (Variables|Default|GetWeaponType)))